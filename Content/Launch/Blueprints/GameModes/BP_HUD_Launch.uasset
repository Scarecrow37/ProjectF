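; Launch-screen HUD that shows an Unreal logo, then a developer logo, as fading splash widgets.
; A reusable Fade macro adds each widget to the viewport, sets logo alpha from a timeline and removes it on finish, chaining the second logo after the first.
; BeginPlay also calls OpenNextLevel on the game mode through BI_NextLevel right after starting the first fade, without waiting for the fades to finish.
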(event EventBeginPlay
  (Utilities|FlowControl|Sequence
    (:then_0
      (bind _returnvalue (UserInterface|CreateWidget "/Game/Launch/Blueprints/UMG/WBP_Unreal.WBP_Unreal_C"))
      (Variables|Default|SetUnreal _returnvalue))
    (:then_1
      (bind _returnvalue_2 (UserInterface|CreateWidget "/Game/Launch/Blueprints/UMG/WBP_Developer.WBP_Developer_C"))
      (Variables|Default|SetDeveloper _returnvalue_2))
    (:then_2
      (Utilities|FlowControl|Sequence
        (:then_0
          (Utilities|Fade (Variables|Default|GetUnreal) (stale _alpha_2) :!label _label
            (:Next
              (Utilities|FlowControl|Sequence
                (:then_0
                  (Utilities|Fade (Variables|Default|GetDeveloper) (stale _alpha) :!label _label_2))
                (:then_1
                  (bind _alpha (Timeline|타임라인 PlayFromStart)
                    (:Update
                      (goto _label_2 Update))
                    (:Finished
                      (goto _label_2 Finish))))))))
        (:then_1
          (bind _alpha_2 (Timeline|ChangeAlpha PlayFromStart)
            (:Update
              (goto _label Update))
            (:Finished
              (goto _label Finish))))))
    (:then_3
      (bind _asbi_next_level (Utilities|Casting|CastToBI_NextLevel (Game|GetGameMode)))
      (Default|OpenNextLevel _asbi_next_level))))

(fn ConstructionScript)